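; Controller builds a 3D grid of block actors when play begins.
; InitData loops over Rows, Cols and Stacks, computes evenly spaced world positions and calls PlaceBlock for each cell.
; PlaceBlock takes a block type, sets the BasicBlock class and spawns it at that position.
; Each spawned block is stored in BlocksMap, keyed by its position vector.
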(event EventBeginPlay
  (CallFunction|InitData))

(event Collision|EventActorBeginOverlap
  (params (OtherActor :type Actor%20Object%20Reference)))

(event EventTick
  (params (DeltaSeconds :type Float%20%28single-precision%29)))

(fn ConstructionScript)

(fn InitData
  ;[1 1 1] InitBlocks
  (for _index (range 1 (LocalVariables|GetRows))
    (for _index_2 (range 1 (LocalVariables|GetCols))
      (for _index_3 (range 1 (LocalVariables|GetStacks))
        (bind _newinstance (CallFunction|PlaceBlock (Math|Vector|MakeVector (* _index 1e+01) (* _index_2 1e+01) (* _index_3 1e+01)) "NewEnumerator0"))
        (Utilities|Map|Add (Variables|Default|GetBlocksMap) (Math|Vector|MakeVector (* _index 1e+01) (* _index_2 1e+01) (* _index_3 1e+01)) _newinstance)))))

(fn PlaceBlock
  (params (Pos :type Vector) (Type :type BlockType%20Enum :default "NewEnumerator0"))
  (switch Utilities|FlowControl|Switch|SwitchonBlockType Type
    (:NewEnumerator0
      (bind _output_get (LocalVariables|SetBlockClass "/Game/Blueprints/Blocks/BasicBlock.BasicBlock_C"))
      (bind _returnvalue (Game|SpawnActorfromClass _output_get (Math|Transform|MakeTransform Pos) "Undefined" "MultiplyWithRoot" 0 0))
      (return _returnvalue))))