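; Basic block actor with a cube mesh that can show a selected or unselected state through its material.
; The construction script creates a dynamic instance of BlockMat on Cube0.
; Select and Unselect toggle the highlight by setting the material's Selected scalar parameter.
; Cursor-over events only forward to the parent class, and nothing in this graph calls the selection functions.
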(event EventBeginPlay)

(event Collision|EventActorBeginOverlap
  (params (OtherActor :type Actor%20Object%20Reference)))

(event EventTick
  (params (DeltaSeconds :type Float%20%28single-precision%29)))

(event MouseInput|EventActorBeginCursorOver
  (|CallParentFunction))

(event MouseInput|EventActorEndCursorOver
  (|CallParentFunction))

(fn ConstructionScript
  (Rendering|Material|CreateDynamicMaterialInstance (Variables|Default|GetCube_0) 0 "/Game/Blueprints/Blocks/BlockMat.BlockMat" "None" :!class /Script/Engine.PrimitiveComponent))

(fn Select
  (Rendering|Material|SetScalarParameterValueonMaterials (Variables|Default|GetCube_0) "Selected" 0.6))

(fn Unselect
  (Rendering|Material|SetScalarParameterValueonMaterials (Variables|Default|GetCube_0) "Selected" 0.0))